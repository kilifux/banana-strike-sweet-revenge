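; BP_BananaPlayerController is a player controller that shows a radial menu while Tab is held.
; It creates a WBP_RadialMenu widget once on BeginPlay and keeps a reference to it.
; Pressing Tab slows global time to half speed, adds the menu, shows the cursor and focuses Game-and-UI input on it.
; Releasing Tab restores normal time, removes the menu, hides the cursor and returns to game-only input.
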(event EventBeginPlay
  (bind _returnvalue (UserInterface|CreateWidget "/Game/Widgets/RadialMenu/WBP_RadialMenu.WBP_RadialMenu_C" self))
  (Variables|Default|SetRadialMenuRef _returnvalue))

(event EventTick
  (params (DeltaSeconds :type Float%20%28single-precision%29)))

(event Input|KeyboardEvents|Tab
  (params (Key :type Key%20Structure :default "None"))
  (bind _radialmenuref (Variables|Default|GetRadialMenuRef))
  (:Pressed
    (Utilities|Time|SetGlobalTimeDilation 0.5)
    (UserInterface|Viewport|AddtoViewport _radialmenuref 0)
    (Variables|Default|SetbShowMouseCursor true)
    (Input|SetInputModeGameandUI self (Variables|Default|GetRadialMenuRef) "DoNotLock" true false))
  (:Released
    (Utilities|Time|SetGlobalTimeDilation 1.0)
    (Widget|RemovefromParent _radialmenuref)
    (Variables|Default|SetbShowMouseCursor false)
    (Input|SetInputModeGameOnly self false)))

(fn ConstructionScript)